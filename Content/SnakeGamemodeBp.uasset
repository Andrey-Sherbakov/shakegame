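; Snake game mode that adds the GUI to the viewport and triggers the win and lose menus.
; BeginPlay binds to the pawn's snake actor destruction, which shows the lose menu through the stored GameInstance variable.
; Tick polls the Elements count and, once it reaches the threshold on Level3, shows the win menu.
; GameInstance is assigned only in that win branch, although the lose handler also relies on it.
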(event Custom|OnDestroyed_Event
  (params (DestroyedActor :type Actor%20Object%20Reference))
  (Default|ShowLoseMenu (Variables|Default|GetGameInstance)))

(event EventBeginPlay
  (bind _returnvalue (UserInterface|CreateWidget "/Game/Interface/GUI.GUI_C" (Game|GetPlayerController 0)))
  (UserInterface|Viewport|AddtoViewport _returnvalue 0)
  (bind _asplayer_pawn_bp (Utilities|Casting|CastToPlayerPawnBp (Game|Player|GetPlayerPawn 0)))
  (Game|AssignOnDestroyed (Variables|/Script/SnakeGame.PlayerPawnBase|GetSnakeActor _asplayer_pawn_bp) (delegate Custom|OnDestroyed_Event)))

(event EventTick
  (params (DeltaSeconds :type Float%20%28single-precision%29))
  (if (>= (Utilities|Array|Length (Variables|Default|GetElements)) 10)
    (bind _returnvalue (Game|GetCurrentLevelName true))
    (if (Utilities|Enum|Equal(Enum) _returnvalue "Level3")
      (bind _assnake_game_instance_bp (Utilities|Casting|CastToSnakeGameInstanceBp (Game|GetGameInstance)))
      (bind _output_get (Variables|Default|SetGameInstance _assnake_game_instance_bp))
      (Default|ShowWinMenu _output_get))))

(fn ConstructionScript)